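; Tracks special notes the player finds and unlocks the ending trigger once five are collected.
; BeginPlay hides and disables the referenced trigger and resets the count, which FindANote increments.
; At the threshold, FindANote re-enables the trigger's collision and tick, shows a "go back to my car" hint on the L1_Character HUD and sets a flag.
; Tick consumes that flag, waits TextDuration, then clears and hides the dialog.
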(event `self.ReceiveBeginPlay`
  (bind _specialnoteendingtrigger (`self.SpecialNoteEndingTrigger`))
  (`self.SetActorHiddenInGame` _specialnoteendingtrigger true)
  (`self.SetActorEnableCollision` _specialnoteendingtrigger false)
  (`self.SetActorTickEnabled` _specialnoteendingtrigger false)
  (set `self.SpecialNotes` 0)
  (set `self.Good` false))

(event `self.ReceiveTick`
  (params (DeltaSeconds :type "Float (single-precision)"))
  (if (`self.Good`)
    (set `self.Good` false)
    (`KismetSystemLibrary.Delay` (`self.TextDuration`))
    (bind _asl1_character (cast `/Game/Blueprints/Game/Level1/L1_Character` (`GameplayStatics.GetPlayerCharacter` 0)))
    (set `/Game/Blueprints/Game/Level1/L1_Character.HintMessage` "" _asl1_character)
    (set `Widget.Visibility` "Hidden" (`/Game/UMG/W_MainHUD.Dialog_Board` (`/Game/Blueprints/Game/Level1/L1_Character.MainHudRef` _asl1_character)))))

(fn `Find a note`
  (bind _specialnoteendingtrigger (`self.SpecialNoteEndingTrigger`))
  (bind _output_get (set `self.SpecialNotes` (+ (`self.SpecialNotes`) 1)))
  (if (>= _output_get 5)
    (`self.SetActorEnableCollision` _specialnoteendingtrigger true)
    (`self.SetActorTickEnabled` _specialnoteendingtrigger true)
    (bind _asl1_character (cast `/Game/Blueprints/Game/Level1/L1_Character` (`GameplayStatics.GetPlayerCharacter` 0)))
    (set `/Game/Blueprints/Game/Level1/L1_Character.HintMessage` "This is too much! I need to leave this place! Right now! I should go back to my car!" _asl1_character)
    (set `Widget.Visibility` "Visible" (`/Game/UMG/W_MainHUD.Dialog_Board` (`/Game/Blueprints/Game/Level1/L1_Character.MainHudRef` _asl1_character)))
    (set `self.Good` true)))

(fn `UserConstructionScript`)