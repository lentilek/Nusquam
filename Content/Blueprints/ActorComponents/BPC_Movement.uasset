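; BPC_Movement is a character component for walk, sprint and crouch movement with stamina.
; Initialize stores the character and sets walk speed, which a helper function changes.
; Its graph holds logic for looping timers that drain and regenerate stamina, and for crouch capsule resizing through L1_Character.
; All six events are empty and that logic is unconnected, so only initialization and the speed setter work as shown.
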(event `StartCrouch`
  ;[1 1 1] Start Crouching
)

(event `StartSprint`
  ;[1 1 1] Start Sprinting
)

(event `EndCrouch`
  ;[1 1 1] End Crouching
)

(event `SprintTimer`
  ;[1 1 1] Sprint Timer
)

(event `StopSprint`
  ;[1 1 1] Stop Sprint
)

(event `RegenerateStamina`
  ;[1 1 1] Regenerate Stamina
)

(fn `Initialize`
  (params (Character :type "Character Object Reference"))
  (set `self.PlayerRef` Character)
  (set `CharacterMovementComponent.MaxWalkSpeed` (`self.WalkSpeed`) (`Character.CharacterMovement` (`self.PlayerRef`))))

(fn `SetPlayerMaxWalkSpeed`
  (params (`Max Walk Speed` :type "Float (single-precision)"))
  (set `CharacterMovementComponent.MaxWalkSpeed` `Max Walk Speed` (`Character.CharacterMovement` (`self.PlayerRef`))))