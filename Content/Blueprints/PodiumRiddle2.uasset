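; Puzzle podium where the player places a required item, revealing its hidden mesh and calling VisibleKey on the linked items riddle.
; An overlap sphere caches the player and inventory, and pressing Action with the wrong item type damages the player.
; While the player is in range, Tick traces to their camera to hide the prompt when blocked, turns it toward the camera, and enables input only within pickup distance.
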(event `self.ReceiveBeginPlay`
  (`SceneComponent.SetVisibility` (`self.StaticMesh`) false false)
  (set `self.CorrectItemHere` false)
  (set `self.CanBePut` false))

(event `InputAction|Action`
  (params (Key :type "Key Structure"))
  (:`Pressed`
    (if (and (`self.CanBePut`) (not (`self.CorrectItemHere`)))
      (if (== (`/Game/Blueprints/ActorComponents/BPC_Inventory.ItemType` (`self.InventoryRef`)) (`self.ItemTypeNeeded`))
        (set `self.CorrectItemHere` true)
        (`SceneComponent.SetVisibility` (`self.StaticMesh`) true false)
        (`SceneComponent.SetVisibility` (`self.PromptWidget`) false false)
        (set `self.UpdateActor` false)
        (`self.DisableInput` (`GameplayStatics.GetPlayerController` 0))
        (`/Game/Blueprints/ItemsRiddle.VisibleKey` (`self.ItemsRiddleRef`))
        (else
          (`GameplayStatics.ApplyDamage` (`self.Player Ref`) (`self.Damage`)))))))

(event `self.Sphere.OnComponentBeginOverlap`
  (params (OverlappedComponent :type "PrimitiveComponent Object Reference") (OtherActor :type "Actor Object Reference") (OtherComp :type "PrimitiveComponent Object Reference") (OtherBodyIndex :type Integer) (bFromSweep :type Boolean) (SweepResult :type "HitResult Structure (by ref)"))
  (if (not (`self.CorrectItemHere`))
    (set `self.CanBePut` true)
    (bind _asl1_character (cast `/Game/Blueprints/Game/Level1/L1_Character` OtherActor))
    (set `self.InventoryRef` (`/Game/Blueprints/Game/Level1/L1_Character.BPC_Inventory` _asl1_character))
    (set `self.Player Ref` _asl1_character)
    (`SceneComponent.SetVisibility` (`self.PromptWidget`) true false)
    (set `self.UpdateActor` true)))

(event `self.Sphere.OnComponentEndOverlap`
  (params (OverlappedComponent :type "PrimitiveComponent Object Reference") (OtherActor :type "Actor Object Reference") (OtherComp :type "PrimitiveComponent Object Reference") (OtherBodyIndex :type Integer))
  (set `self.CanBePut` false)
  (cast `/Game/Blueprints/Game/Level1/L1_Character` OtherActor)
  (`SceneComponent.SetVisibility` (`self.PromptWidget`) false false)
  (set `self.UpdateActor` false)
  (`self.DisableInput` (`GameplayStatics.GetPlayerController` 0)))

(event `self.ReceiveTick`
  (params (DeltaSeconds :type "Float (single-precision)"))
  (bind _returnvalue (`GameplayStatics.GetPlayerController` 0))
  (bind _promptwidget (`self.PromptWidget`))
  (bind _camera (`/Game/Blueprints/Game/Level1/L1_Character.Camera` (`self.Player Ref`)))
  (if (and (`self.UpdateActor`) (not (`self.CorrectItemHere`)))
    (bind (_outhit _returnvalue_2) (`KismetSystemLibrary.LineTraceSingle` (`self.K2_GetActorLocation`) (`SceneComponent.K2_GetComponentLocation` _camera) "TraceTypeQuery1"))
    (if _returnvalue_2
      (`SceneComponent.SetVisibility` _promptwidget false false)
      (`self.DisableInput` (`GameplayStatics.GetPlayerController` 0))
      (else
        (`SceneComponent.SetVisibility` _promptwidget true false)
        (`SceneComponent.K2_SetWorldRotation` _promptwidget (`KismetMathLibrary.FindLookAtRotation` (`SceneComponent.K2_GetComponentLocation` _promptwidget) (`SceneComponent.K2_GetComponentLocation` _camera)) false false)
        (bind _asw_pickup_prompt (cast `/Game/UMG/W_PickupPrompt` (`WidgetComponent.GetUserWidgetObject` _promptwidget)))
        (bind (_bblockinghit _binitialoverlap _time _distance _location _impactpoint _normal _impactnormal _physmat _hitactor _hitcomponent _hitbonename _bonename _hititem _elementindex _faceindex _tracestart _traceend) (`GameplayStatics.BreakHitResult` _outhit))
        (bind _returnvalue_3 (<= (`KismetMathLibrary.VSize` (- _tracestart _traceend)) (`self.PickUpDistance`)))
        (`/Game/UMG/W_PickupPrompt.TogglePrompt` _asw_pickup_prompt _returnvalue_3)
        (if _returnvalue_3
          (`self.EnableInput` _returnvalue)
          (else
            (`self.DisableInput` _returnvalue)))))))

(fn `UserConstructionScript`)