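; Trigger actor that shows the opening story monologue about the dead engine and the woods when the player overlaps it.
; On begin overlap it casts to L1_Character, sets its HintMessage text and makes the main HUD's DialogBoard visible.
; On end overlap it clears the message, hides the board and destroys itself, so the hint plays only once.
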(event `self.ReceiveActorBeginOverlap`
  (params (OtherActor :type "Actor Object Reference"))
  (bind _asl1_character (cast `/Game/Blueprints/Game/Level1/L1_Character` OtherActor))
  (set `/Game/Blueprints/Game/Level1/L1_Character.HintMessage` "Of course. Middle of nowhere, radio dead, and now this. The engine just died like it saw a ghost. Or maybe it smelled one. Either way... I’m not walking back through those woods." _asl1_character)
  (set `Widget.Visibility` "Visible" (`/Game/UMG/W_MainHUD.Dialog_Board` (`/Game/Blueprints/Game/Level1/L1_Character.MainHudRef` _asl1_character))))

(event `self.ReceiveActorEndOverlap`
  (params (OtherActor :type "Actor Object Reference"))
  (bind _asl1_character (cast `/Game/Blueprints/Game/Level1/L1_Character` OtherActor))
  (set `/Game/Blueprints/Game/Level1/L1_Character.HintMessage` "" _asl1_character)
  (set `Widget.Visibility` "Hidden" (`/Game/UMG/W_MainHUD.Dialog_Board` (`/Game/Blueprints/Game/Level1/L1_Character.MainHudRef` _asl1_character)))
  (`self.K2_DestroyActor`))

(fn `UserConstructionScript`)