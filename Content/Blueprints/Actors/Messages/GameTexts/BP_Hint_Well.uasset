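; Hint trigger actor for the well, telling the player that an inscription asks for four keys to move on.
; On overlap by L1_Character, it sets that character's HintMessage and shows the DialogBoard on its main HUD.
; When the character leaves, it clears the message, hides the board and destroys itself, so the hint appears only once.
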(event `self.ReceiveActorBeginOverlap`
  (params (OtherActor :type "Actor Object Reference"))
  (bind _asl1_character (cast `/Game/Blueprints/Game/Level1/L1_Character` OtherActor))
  (set `/Game/Blueprints/Game/Level1/L1_Character.HintMessage` "Hmmm on the well that inscription is probably.... Bring four keys to move on.... I think this farther is about this church? Well, let's look for those keys…" _asl1_character)
  (set `Widget.Visibility` "Visible" (`/Game/UMG/W_MainHUD.Dialog_Board` (`/Game/Blueprints/Game/Level1/L1_Character.MainHudRef` _asl1_character))))

(event `self.ReceiveActorEndOverlap`
  (params (OtherActor :type "Actor Object Reference"))
  (bind _asl1_character (cast `/Game/Blueprints/Game/Level1/L1_Character` OtherActor))
  (set `/Game/Blueprints/Game/Level1/L1_Character.HintMessage` "" _asl1_character)
  (set `Widget.Visibility` "Hidden" (`/Game/UMG/W_MainHUD.Dialog_Board` (`/Game/Blueprints/Game/Level1/L1_Character.MainHudRef` _asl1_character)))
  (`self.K2_DestroyActor`))

(fn `UserConstructionScript`)