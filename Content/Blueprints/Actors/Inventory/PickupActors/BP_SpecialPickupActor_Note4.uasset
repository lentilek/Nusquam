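; Special note pickup actor, apparently the fourth note variant, that puts its item into the player's inventory when the Action input is pressed.
; A press notifies SpecialNote through FindANote, calls AddItem on the player's inventory component and plays a pickup sound, all before checking success.
; On success it keeps any remainder as its new amount or destroys itself.
; Construction defers to the parent class.
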(event `InputAction|Action`
  (params (Key :type "Key Structure"))
  (:`Pressed`
    (`/Game/Blueprints/SpecialNotes.Find a note` (`self.SpecialNote`))
    (bind (_success_ _remainder) (`/Game/Blueprints/ActorComponents/BPC_Inventory.AddItem` (`/Game/Blueprints/Game/Level1/L1_Character.BPC_Inventory` (`self.Player Ref`)) (`self.Item`) (`self.Amount`)))
    (`GameplayStatics.PlaySoundAtLocation` "/Game/Audio/interactions/pick_up.pick_up" (`self.K2_GetActorLocation`) (struct) 1.0 1.0 0.0 null null null null)
    (if _success_
      (if (> _remainder 0)
        (set `self.Amount` _remainder)
        (else
          (`self.K2_DestroyActor`))))))

(fn `UserConstructionScript`
  (`parent.UserConstructionScript`))