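; BP_PickupActor_Note1 is a note pickup actor that stays hidden until the player has collected enough keys.
; On BeginPlay it caches the player as L1_Character and hides itself, provided that cast succeeds.
; Every Tick it polls the character's KeyCollected count and unhides itself once the count reaches four or more.
; Any pickup behavior comes from its parent class, as this Blueprint only adds the visibility gate.
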(event `self.ReceiveBeginPlay`
  (`parent.ReceiveBeginPlay`)
  (bind _asl1_character (cast `/Game/Blueprints/Game/Level1/L1_Character` (`GameplayStatics.GetPlayerCharacter` 0)))
  (set `self.PlayerRef` _asl1_character)
  (`self.SetActorHiddenInGame` true))

(event `self.ReceiveTick`
  (params (DeltaSeconds :type "Float (single-precision)"))
  (`parent.ReceiveTick` DeltaSeconds)
  (if (>= (`/Game/Blueprints/Game/Level1/L1_Character.KeyCollected` (`self.PlayerRef`)) 4)
    (`self.SetActorHiddenInGame` false)))

(fn `UserConstructionScript`
  (`parent.UserConstructionScript`))