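; ItemsRiddle is a puzzle controller that reveals a key once three podiums each hold their correct item.
; On BeginPlay it hides the referenced Key actor and disables its collision and tick.
; The VisibleKey function checks the CorrectItemHere flag on all three podium references and, if all are true, restores the key's visibility, collision and tick.
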(event `self.ReceiveBeginPlay`
  (bind _key (`self.Key`))
  (`self.SetActorHiddenInGame` _key true)
  (`self.SetActorEnableCollision` _key false)
  (`self.SetActorTickEnabled` _key false))

(event `self.ReceiveTick`
  (params (DeltaSeconds :type "Float (single-precision)")))

(fn `UserConstructionScript`)

(fn `VisibleKey`
  (bind _key (`self.Key`))
  (if (and (`/Game/Blueprints/PodiumRiddle.CorrectItemHere` (`self.PodiumRiddle1`)) (`/Game/Blueprints/PodiumRiddle2.CorrectItemHere` (`self.PodiumRiddle2`)) (`/Game/Blueprints/PodiumRiddle3.CorrectItemHere` (`self.PodiumRiddle3`)))
    (`self.SetActorHiddenInGame` _key false)
    (`self.SetActorEnableCollision` _key true)
    (`self.SetActorTickEnabled` _key true)))